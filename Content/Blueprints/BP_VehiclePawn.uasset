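; Vehicle pawn Blueprint that animates the visual rotation of its four wheels.
; Each Tick accumulates a shared roll angle from CurrentSpeed, without delta-time scaling, and applies it as relative pitch to every wheel.
; The front wheels also yaw by half of CurrentSteering, while the rear wheels only roll.
; The graph only reads speed and steering; it contains no movement or input logic.
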(event EventBeginPlay)

(event Collision|EventActorBeginOverlap
  (params (OtherActor :type Actor%20Object%20Reference)))

(event EventTick
  (params (DeltaSeconds :type Float%20%28single-precision%29))
  ;[0.15 0.15 0.15 0.5] Calcul du roulement des roues, il augmente a chaque frame en fonction de la vitesse actuelle du véhicule
  (bind _output_get (Variables|Default|SetWheelRoll (- (Variables|Default|GetWheelRoll) (* (Variables|Default|GetCurrentSpeed) 0.05))))
  ;[0.15 0.15 0.15 0.5] Rotation des roues avant avec roulement en Y et direction en Z
  (Transformation|SetRelativeRotation (Variables|Default|GetForwardRightWheel) (Math|Rotator|MakeRotator 0.0 _output_get (/ (Variables|Default|GetCurrentSteering) 2.0)) false false)
  (Transformation|SetRelativeRotation (Variables|Default|GetForwardLeftWheel) (Math|Rotator|MakeRotator 0.0 _output_get (/ (Variables|Default|GetCurrentSteering) 2.0)) false false)
  ;[0.15 0.15 0.15 0.5] Rotation des roues arrières uniquement en Y pour le roulement
  (Transformation|SetRelativeRotation (Variables|Default|GetBackLeftWheel) (Math|Rotator|MakeRotator 0.0 (Variables|Default|GetWheelRoll) 0.0) false false)
  (Transformation|SetRelativeRotation (Variables|Default|GetBackRightWheel) (Math|Rotator|MakeRotator 0.0 (Variables|Default|GetWheelRoll) 0.0) false false))

(fn ConstructionScript)